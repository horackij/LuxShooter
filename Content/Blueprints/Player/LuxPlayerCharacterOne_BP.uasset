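; Player character Blueprint that sets up the starting weapon loadout and handles weapon switching.
; On BeginPlay, after the parent logic, it grants the base weapon as equipped and blue, green, red and purple variants unequipped.
; Mouse wheel up and down call CycleWeapons in opposite directions.
; The weapon logic itself lives outside these graphs, and the construction script only calls its parent.
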(event EventBeginPlay
  (|CallParentFunction)
  (Class|LuxCharacterBase|GrantWeapon "/Game/Blueprints/Weapons/WeaponBase_BP.WeaponBase_BP_C" true)
  (Class|LuxCharacterBase|GrantWeapon "/Game/Blueprints/Weapons/WeaponBaseBlue_BP.WeaponBaseBlue_BP_C" false)
  (Class|LuxCharacterBase|GrantWeapon "/Game/Blueprints/Weapons/WeaponBaseGreen_BP.WeaponBaseGreen_BP_C" false)
  (Class|LuxCharacterBase|GrantWeapon "/Game/Blueprints/Weapons/WeaponBaseRed_BP.WeaponBaseRed_BP_C" false)
  (Class|LuxCharacterBase|GrantWeapon "/Game/Blueprints/Weapons/WeaponBasePuple_BP.WeaponBasePuple_BP_C" false))

(event Collision|EventActorBeginOverlap
  (params (OtherActor :type Actor%20Object%20Reference)))

(event EventTick
  (params (DeltaSeconds :type Float%20%28single-precision%29)))

(event Input|MouseEvents|MouseWheelUp
  (params (Key :type Key%20Structure :default "None"))
  (:Pressed
    (Class|LuxCharacterBase|CycleWeapons true)))

(event Input|MouseEvents|MouseWheelDown
  (params (Key :type Key%20Structure :default "None"))
  (:Pressed
    (Class|LuxCharacterBase|CycleWeapons false)))

(fn ConstructionScript
  (|CallParentFunction))