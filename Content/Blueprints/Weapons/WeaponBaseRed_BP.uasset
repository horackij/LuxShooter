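; Red weapon Blueprint that extends a parent weapon class, supplying its firing effects and equip visuals.
; Start and stop firing defer to the parent, while each fired round plays a shot sound and spawns a tiny explosion emitter at the muzzle point.
; Equipping reveals the skeletal mesh after a short delay; unequipping hides it after a delay and destroys the actor.
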(event EventBeginPlay)

(event Collision|EventActorBeginOverlap
  (params (OtherActor :type Actor%20Object%20Reference)))

(event EventTick
  (params (DeltaSeconds :type Float%20%28single-precision%29)))

(event EventStartFiring
  (|CallParentFunction))

(event EventStopFiring
  (|CallParentFunction))

(event EventOnFiredRound
  (bind _muzzlepoint (Variables|Default|GetMuzzlePoint))
  (bind _returnvalue (Transformation|GetWorldLocation _muzzlepoint))
  (Audio|PlaySoundatLocation "/Game/FirstPerson/Audio/FirstPersonTemplateWeaponFire02.FirstPersonTemplateWeaponFire02" _returnvalue "0, 0, 0" 0.5 1.0 0.0 0 0 0)
  (Effects|SpawnEmitteratLocation "/Game/StarterContent/Particles/P_Explosion.P_Explosion" _returnvalue "0, 0, 0" "0.050000,0.050000,0.050000"))

(event EventOnEquipped
  (Utilities|FlowControl|Delay 1.0)
  (Rendering|SetVisibility (Variables|Default|GetSkeletalMesh) true false))

(event EventOnUnequipped
  (Utilities|FlowControl|Delay 0.5)
  (Rendering|SetVisibility (Variables|Default|GetSkeletalMesh) false false)
  (Actor|DestroyActor))

(fn ConstructionScript)